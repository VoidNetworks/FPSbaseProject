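; First-person character controller with look, movement, walk, crouch, double jump, dash and recall abilities.
; Dash briefly launches the character along the camera's forward vector, then stops it and waits out a cooldown.
; Tick samples transforms on a delay into a debug-drawn list, removing the newest entry at eight.
; Recall pauses sampling and lerps location and control rotation back through that list to its first entry, then clears it and cools down.
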(event `InputAxis|MouseLookHorizontal`
  (params (AxisValue :type "Float (single-precision)"))
  ;[1 1 1] MouseInputs
  (`self.AddControllerYawInput` AxisValue))

(event `InputAxis|Horizontal`
  (params (AxisValue :type "Float (single-precision)"))
  (bind (_returnvalue_roll _returnvalue_pitch _returnvalue_yaw) (`KismetMathLibrary.BreakRotator` (`self.GetControlRotation`)))
  ;[1 1 1] MovementsInputs
  (`self.AddMovementInput` (`KismetMathLibrary.GetRightVector` (`KismetMathLibrary.MakeRotator` 0.0 0.0 _returnvalue_yaw)) AxisValue))

(event `InputAxis|MouseLookVertical`
  (params (AxisValue :type "Float (single-precision)"))
  ;[1 1 1] MouseInputs
  (`self.AddControllerPitchInput` AxisValue))

(event `InputAxis|Vertical`
  (params (AxisValue :type "Float (single-precision)"))
  (bind (_returnvalue_roll _returnvalue_pitch _returnvalue_yaw) (`KismetMathLibrary.BreakRotator` (`self.GetControlRotation`)))
  ;[1 1 1] MovementsInputs
  (`self.AddMovementInput` (`KismetMathLibrary.GetForwardVector` (`KismetMathLibrary.MakeRotator` 0.0 0.0 _returnvalue_yaw)) AxisValue))

(event `InputAction|Jump`
  (params (Key :type "Key Structure"))
  ;[1 1 1] MovementsInputs
  (:`Pressed`
    (bind _counter (`/Engine/EditorBlueprintResources/StandardMacros.Do N` 2 :!label _label)
      (:`Exit`
        (switch `int` _counter
          (:`1`
            (`self.Jump`))
          (:`2`
            (`self.LaunchCharacter` (0.0 0.0 800.0))))))))

(event `self.OnLanded`
  (params (Hit :type "HitResult Structure (by ref)"))
  ;[1 1 1] MovementsInputs
  (goto _label :!via `Reset`))

(event `InputAction|Walk`
  (params (Key :type "Key Structure"))
  (bind _charactermovement (`self.CharacterMovement`))
  ;[1 1 1] MovementsInputs
  (:`Pressed`
    (set `CharacterMovementComponent.MaxWalkSpeed` 300.0 _charactermovement))
  (:`Released`
    (set `CharacterMovementComponent.MaxWalkSpeed` 600.0 _charactermovement)))

(event `InputAction|Crouch`
  (params (Key :type "Key Structure"))
  ;[1 1 1] MovementsInputs
  (:`Pressed`
    (`self.Crouch`))
  (:`Released`
    (`self.UnCrouch`)))

(event `InputAction|Dash`
  (params (Key :type "Key Structure"))
  ;[1 1 1] Abilities
  ;;[1 1 1] Dash Ability
  (:`Pressed`
    (if (`self.CanDash?`)
      (`self.LaunchCharacter` (* (`SceneComponent.GetForwardVector` (`self.Camera`)) 20000.0))
      (`KismetSystemLibrary.Delay` 0.03)
      (set `self.CanDash?` false)
      (`MovementComponent.StopMovementImmediately` (`self.CharacterMovement`))
      (`KismetSystemLibrary.Delay` 1.0)
      (set `self.CanDash?` true))))

(event `self.ReceiveTick`
  (params (DeltaSeconds :type "Float (single-precision)"))
  (bind _returnvalue (`GameplayStatics.GetPlayerController` 0))
  (bind _counter (`self.Counter`))
  (bind _recallpositions (`self.RecallPositions`))
  (bind _recallpositions_2 (`self.RecallPositions`))
  (bind _output (`|GetArrayItem` (`self.RecallPositions`) _counter))
  (bind (_returnvalue_location _returnvalue_rotation) (`KismetMathLibrary.BreakTransform` (`KismetMathLibrary.TLerp` (`self.GetTransform`) _output (* (`self.DeltaTime`) (`self.TravelSpeed`)))))
  ;[1 1 1] Abilities
  ;;[1 1 1] Recall Ability
  (set `self.DeltaTime` DeltaSeconds)
  (`|ExecutionSequence`
    (:`then_0`
      (if (`self.CanSetPos?`)
        (`KismetSystemLibrary.Delay` (`self.TimeBeforeSettingNewPos`))
        (if (>= (`KismetArrayLibrary.Array_Length` _recallpositions) 8)
          (`KismetArrayLibrary.Array_Remove` _recallpositions (`KismetArrayLibrary.Array_LastIndex` _recallpositions))
          (else
            (bind _returnvalue_2 (`KismetArrayLibrary.Array_Add` _recallpositions_2 (`self.GetTransform`)))
            (`KismetSystemLibrary.DrawDebugFrustum` (`|GetArrayItem` _recallpositions_2 _returnvalue_2) (struct :`R` 1.0 :`G` 0.185487 :`A` 1.0) 6.0 15.0)))))
    (:`then_1`
      (if (`self.RecallPressed`)
        (`self.K2_SetActorLocation` _returnvalue_location)
        (`Controller.SetControlRotation` _returnvalue (`KismetMathLibrary.RLerp` (`self.K2_GetActorRotation` _returnvalue) _returnvalue_rotation (* (`self.DeltaTime`) (`self.RotationSpeed`))))
        (if (`KismetMathLibrary.NearlyEqual_TransformTransform` (`self.GetTransform`) _output 120.0 120.0 120.0)
          (if (== _counter 0)
            (set `self.CanSetPos?` true)
            (set `self.RecallPressed` false)
            (`KismetArrayLibrary.Array_Clear` (`self.RecallPositions`))
            (`KismetSystemLibrary.Delay` 6.0)
            (set `self.CanRecall?` true)
            (else
              (`/Engine/EditorBlueprintResources/StandardMacros.DecrementInt` (`self.Counter`)))))))))

(event `InputAction|Recall`
  (params (Key :type "Key Structure"))
  ;[1 1 1] Abilities
  ;;[1 1 1] Recall Ability
  (:`Pressed`
    (if (`self.CanRecall?`)
      (set `self.RecallPressed` true)
      (set `self.CanRecall?` false)
      (set `self.CanSetPos?` false)
      (set `self.Counter` (`KismetArrayLibrary.Array_LastIndex` (`self.RecallPositions`))))))

(fn `UserConstructionScript`)